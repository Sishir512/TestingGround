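; AI controller for guard NPCs that switches them between patrol and shooting based on perception.
; On begin play it sets up the PatrolData blackboard, runs the GuardBehaviour tree and caches its controlled character.
; Perception updates on actors lacking the "Enemy" tag set or clear the blackboard's enemy key and toggle the controller's Alerted flag and the guard's Shooting flag.
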(event `self.ReceiveBeginPlay`
  (bind _blackboardcomponent (`self.UseBlackboard` "/Game/Dynamic/Character/AI/PatrolData.PatrolData"))
  (set `self.BlackBoardComp` _blackboardcomponent)
  (`self.RunBehaviorTree` "/Game/Dynamic/Character/AI/GuardBehaviour.GuardBehaviour")
  (bind _ascharacter (cast `/Game/Dynamic/Character/Behavior/Character` (`self.K2_GetPawn`)))
  (set `self.PatrollingGuard` _ascharacter))

(event `self.AIPerception.OnTargetPerceptionUpdated`
  (params (Actor :type "Actor Object Reference") (Stimulus :type "AIStimulus Structure"))
  (bind _patrollingguard (`self.PatrollingGuard`))
  (bind _blackboardcomp (`self.BlackBoardComp`))
  (bind _enemykey (`self.EnemyKey`))
  (if (`self.ActorHasTag` Actor "Enemy")
    _
    (elif (`.bSuccessfullySensed` (break `AIStimulus` Stimulus))
      (`BlackboardComponent.SetValueAsObject` _blackboardcomp _enemykey Actor)
      (set `self.Alerted` true)
      (set `/Game/Dynamic/Character/Behavior/Character.Shooting` true _patrollingguard)
      (else
        (`BlackboardComponent.ClearValue` _blackboardcomp _enemykey)
        (set `self.Alerted` false)
        (set `/Game/Dynamic/Character/Behavior/Character.Shooting` false _patrollingguard)))))

(fn `UserConstructionScript`)