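; Game mode for an infinite terrain game that spawns chained tiles and keeps the player's score.
; On BeginPlay it populates a pool of nav mesh bounds volumes, then spawns a starting run of tiles.
; Each SpawnTile call passes the pool to the new tile and stores that tile's attach location as the next spawn transform.
; IncreaseScore and ReturnScore increment and expose the score.
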(event `self.ReceiveBeginPlay`
  (`self.PopulateBoundsVolume`)
  (for _ (range 4)
    (`self.SpawnTile`)))

(fn `IncreaseScore`
  (`/Engine/EditorBlueprintResources/StandardMacros.IncrementInt` (`self.Score`)))

(fn `ReturnScore`
  (returns (NewParam :type Integer))
  (return (`self.Score`)))

(fn `SpawnTile`
  (returns (NewParam :type "/Game/Dynamic/Terrain/BPTile Object Reference"))
  (bind _returnvalue (`|SpawnActorFromClass` "/Game/Dynamic/Terrain/BPTile.BPTile_C" (`self.NextTileTransform`) "Undefined" "OverrideRootScale" null null))
  (`Tile.SetPool` _returnvalue (`self.NavMeshBoundsVolumePool`))
  (bind _attachtransform (`/Game/Dynamic/Terrain/BPTile.GetAttachLocation` _returnvalue))
  (set `self.NextTileTransform` _attachtransform)
  (return _returnvalue))

(fn `UserConstructionScript`)